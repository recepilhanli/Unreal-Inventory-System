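; Player character Blueprint handling local UI, jumping and movement-based camera shake.
; The local player gets quick inventory and HUD widgets on BeginPlay, while non-local instances disable Tick after a short delay.
; Tick classifies movement as idle or airborne, walking or running from velocity and max walk speed, then feeds that state to PlayShake.
; Tab opens or closes the backpack, and a look-at event shows or removes the collectible item widget.
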(event `self.ReceiveBeginPlay`
  (if (`self.IsLocallyControlled`)
    (bind _returnvalue (`|CreateWidget` "/Game/Misc/UI/Backpack-inventory/QuickInventoryUI.QuickInventoryUI_C"))
    (bind _returnvalue_2 (`|CreateWidget` "/Game/Misc/UI/HUD/PlayerHUD.PlayerHUD_C"))
    (`UserWidget.AddToViewport` _returnvalue 0)
    (`UserWidget.AddToViewport` _returnvalue_2 0)
    (else
      (`KismetSystemLibrary.Delay` 1.0)
      (`self.SetActorTickEnabled` false))))

(event `self.ReceiveTick`
  (params (DeltaSeconds :type "Float (single-precision)"))
  (bind _state (`self.GetPlayerState`))
  (`/Game/Blueprints/Player/PlayerShake.PlayShake` (`KismetMathLibrary.Conv_ByteToInt` _state) (`GameplayStatics.GetPlayerController` 0)))

(event `Key|C`
  (params (Key :type "Key Structure"))
  (:`Pressed`
    (`self.Jump`))
  (:`Released`
    (`self.StopJumping`)))

(event `Key|Tab`
  (params (Key :type "Key Structure"))
  (bind _inventory (`self.Inventory`))
  (:`Pressed`
    (if (`PlayerInventory.InBackpack` _inventory)
      (`Widget.RemoveFromParent` (`PlayerInventory.BackpackWidget` _inventory))
      (else
        (bind _returnvalue (`|CreateWidget` "/Game/Misc/UI/Backpack-inventory/BackpackUI.BackpackUI_C"))
        (`UserWidget.AddToViewport` _returnvalue 0)
        (set `PlayerController.bShowMouseCursor` true (`GameplayStatics.GetPlayerController` 0))))))

(event `self.PlayerLookingItemEvent`
  (params (onscreen :type Boolean) (item :type "ItemData Object Reference"))
  (bind _collectiblewidget (`PlayerInventory.CollectibleWidget` (`self.Inventory`)))
  (if onscreen
    (if (not (`KismetSystemLibrary.IsValid` _collectiblewidget))
      (bind _returnvalue (`|CreateWidget` "/Game/Misc/UI/Backpack-inventory/CollectiableItem.CollectiableItem_C" null item))
      (`UserWidget.AddToViewport` _returnvalue 0))
    (else
      (`/Engine/EditorBlueprintResources/StandardMacros.IsValid` _collectiblewidget
        (:`Is Valid`
          (`Widget.RemoveFromParent` _collectiblewidget))))))

(fn `GetPlayerState`
  (returns (State :type Byte))
  (bind _charactermovement (`self.CharacterMovement`))
  (if (and (> (`KismetMathLibrary.VSize` (`MovementComponent.Velocity` _charactermovement)) 2.0) (!= (`NavMovementComponent.IsFalling` _charactermovement) true))
    (if (> (`CharacterMovementComponent.MaxWalkSpeed` _charactermovement) 500.0)
      (return 2)
      (else
        (return 1)))
    (else
      (return 0))))

(fn `UserConstructionScript`)